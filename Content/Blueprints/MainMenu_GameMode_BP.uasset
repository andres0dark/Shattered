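; Main menu game mode that sets up local multiplayer player registration on BeginPlay.
; It creates extra local players up to MaxPlayers, then shows the MainMenu widget owned by the first controller.
; Each player gets a PlayerCustomization widget in the menu's RegisterArea, which is also stored on that player's MainMenu_PlayerController_BP as its Menu.
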(event EventBeginPlay
  (for _index (range 1 (- (Variables|Default|GetMaxPlayers) 1))
    (Class|GameplayStatics|CreatePlayer _index))
  (bind _returnvalue (UserInterface|CreateWidget "/Game/UI/MainMenu.MainMenu_C" (Game|GetPlayerController 0)))
  (bind _output_get (Variables|Default|SetMainMenuWidget _returnvalue))
  (UserInterface|Viewport|AddtoViewport _output_get 0)
  (for _index_2 (range 0 (- (Variables|Default|GetMaxPlayers) 1))
    (bind _returnvalue_2 (UserInterface|CreateWidget "/Game/UI/PlayerCustomization.PlayerCustomization_C" (Game|GetPlayerController _index_2)))
    (Widget|Panel|AddChild (Variables|/Game/UI/MainMenu.MainMenu_C|GetRegisterArea (Variables|Default|GetMainMenuWidget)) _returnvalue_2)
    (bind _asmain_menu_player_controller_bp (Utilities|Casting|CastToMainMenu_PlayerController_BP (Game|GetPlayerController _index_2)))
    (Variables|/Game/Blueprints/MainMenu_PlayerController_BP.MainMenu_PlayerController_BP_C|SetMenu _asmain_menu_player_controller_bp _returnvalue_2)))

(fn ConstructionScript)