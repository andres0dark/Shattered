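; Player controller for the hammer attack that previews and shatters destructible blocks near the pawn.
; While hammering, Tick traces from the block below along facing snapped to 45-degree steps, tinting hit blocks in the player's color and restoring previous ones.
; A looping timer lengthens the trace up to a cap, used only for cardinal directions; diagonals stay fixed.
; BreakBlocks stops the timer, damages highlighted blocks, makes them physics-only and resets their color.
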(event Custom|StopHammering_BP
  (Variables|Default|SetDrawHammerVector false))

(event Custom|StartHammering_BP
  (Variables|Default|SetDrawHammerVector true)
  (Variables|Default|Setbreak_length 175.0)
  (bind _returnvalue (Utilities|Time|SetTimerbyFunctionName 0 "BreakLength" 0.1 true)))

(event Custom|BreakBlocks
  (Utilities|Time|ClearandInvalidateTimerbyHandle (stale Custom|StartHammering_BP _returnvalue))
  (for _array_element (Variables|Default|GetHitBlocks)
    (bind _asdestructible_component (Utilities|Casting|CastToDestructibleComponent _array_element))
    (Class|DestructibleComponent|ApplyDamage _asdestructible_component 3e+01 (+ (Transformation|GetActorLocation (Components|GetOwner _array_element)) (* (Math|Vector|GetUnitDirection(Vector) (Transformation|GetActorLocation (Components|GetOwner _array_element)) (Transformation|GetActorLocation (Pawn|GetControlledPawn))) 100)) (Math|Vector|MakeVector 0.0 0.0 -1.0) 3e+03)
    (Collision|SetCollisionEnabled _asdestructible_component "PhysicsOnly")
    (bind _returnvalue (Rendering|Material|CreateDynamicMaterialInstance _asdestructible_component 0 0 "None" :!class /Script/Engine.PrimitiveComponent))
    (Rendering|Material|SetVectorParameterValue _returnvalue "Color" (Math|Conversions|ToLinearColor(Vector) "0.574409,0.582118,0.630208") :!class /Script/Engine.MaterialInstanceDynamic)))

(event EventBeginPlay
  (Utilities|Array|Clear (Variables|Default|GetHitBlocks))
  (Utilities|Array|Clear (Variables|Default|GetOldHitBlocks)))

(event EventTick
  (params (DeltaSeconds :type Float%20%28single-precision%29))
  (bind _returnvalue (Math|Float|MultiplybyPi 0.25))
  (bind _returnvalue_2 (Pawn|GetControlledPawn))
  (bind _oldhitblocks (Variables|Default|GetOldHitBlocks))
  (bind _returnvalue_3 (Transformation|GetActorForwardVector _returnvalue_2))
  (bind _returnvalue_4 (Transformation|GetActorLocation _returnvalue_2))
  (bind (_x _y _z) (Math|Vector|BreakVector _returnvalue_3))
  (bind (_x_2 _y_2) (Math|Vector|BreakVector _returnvalue_4))
  (bind _returnvalue_5 (Math|Trig|Acos(Degrees) _x))
  (bind _returnvalue_6 (Class|KismetMathLibrary|Asin _y))
  (bind _returnvalue_7 (Math|Float|Min(Float) _z 0.0))
  (bind _returnvalue_8 (/ _returnvalue_6 _returnvalue))
  (bind _returnvalue_9 (/ _returnvalue_5 _returnvalue))
  (bind _returnvalue_10 (Math|Float|Round _returnvalue_8))
  (bind _returnvalue_11 (Math|Float|Round _returnvalue_9))
  (bind _returnvalue_12 (* _returnvalue_10 _returnvalue))
  (bind _returnvalue_13 (* _returnvalue_11 _returnvalue))
  (bind _returnvalue_14 (Math|Trig|Cos(Radians) _returnvalue_13))
  (bind _returnvalue_15 (Math|Trig|Sin(Radians) _returnvalue_12))
  (bind _returnvalue_16 (Math|Vector|MakeVector _returnvalue_14 _returnvalue_15 _returnvalue_7))
  (bind _returnvalue_17 (Math|Float|Absolute(Float) _returnvalue_14))
  (bind _returnvalue_18 (Math|Float|Absolute(Float) _returnvalue_15))
  (if (Variables|Default|GetDrawHammerVector)
    (bind _outhit (Collision|LineTraceByChannel _returnvalue_4 (Math|Vector|MakeVector _x_2 _y_2 0.0) "TraceTypeQuery1" false 0 "None"))
    (if (.bBlockingHit (Collision|BreakHitResult _outhit))
      (bind _outhits (Collision|MultiLineTraceByChannel (+ (Math|Vector|MakeVector (.X (Math|Vector|BreakVector (Transformation|GetActorLocation (.HitActor (Collision|BreakHitResult _outhit))))) (.Y (Math|Vector|BreakVector (Transformation|GetActorLocation (.HitActor (Collision|BreakHitResult _outhit))))) (Math|Float|Min(Float) (.Z (Math|Vector|BreakVector _returnvalue_4)) 0.0)) (* _returnvalue_16 2.5e+02)) (+ (Math|Vector|MakeVector (.X (Math|Vector|BreakVector (Transformation|GetActorLocation (.HitActor (Collision|BreakHitResult _outhit))))) (.Y (Math|Vector|BreakVector (Transformation|GetActorLocation (.HitActor (Collision|BreakHitResult _outhit))))) (Math|Float|Min(Float) (.Z (Math|Vector|BreakVector _returnvalue_4)) 0.0)) (* _returnvalue_16 (Math|Float|SelectFloat (Variables|Default|Getbreak_length) 2e+02 (and (or (>= _returnvalue_17 0.95) (<= _returnvalue_17 0.05)) (or (>= _returnvalue_18 0.95) (<= _returnvalue_18 0.05)))))) "TraceTypeQuery3" false 0 "None"))
      (Utilities|Array|Clear (Variables|Default|GetHitBlocks))
      (for _array_element _outhits
        (Utilities|Array|AddUnique (Variables|Default|GetHitBlocks) (.HitComponent (Collision|BreakHitResult _array_element)))
        (bind _returnvalue_19 (Rendering|Material|CreateDynamicMaterialInstance (.HitComponent (Collision|BreakHitResult _array_element)) 0 0 "None" :!class /Script/Engine.PrimitiveComponent))
        (bind _asshattered_character_bp (Utilities|Casting|CastToShatteredCharacter_BP (Pawn|GetControlledPawn)))
        (Rendering|Material|SetVectorParameterValue _returnvalue_19 "Color" (Variables|/Game/PlayerCharacter/ShatteredCharacter_BP.ShatteredCharacter_BP_C|GetPlayerColor _asshattered_character_bp) :!class /Script/Engine.MaterialInstanceDynamic))
      (for _array_element_2 (Variables|Default|GetHitBlocks)
        (Utilities|Array|RemoveItem (Variables|Default|GetOldHitBlocks) _array_element_2))
      (for _array_element_3 (Variables|Default|GetOldHitBlocks)
        (bind _returnvalue_20 (Rendering|Material|CreateDynamicMaterialInstance _array_element_3 0 0 "None" :!class /Script/Engine.PrimitiveComponent))
        (Rendering|Material|SetVectorParameterValue _returnvalue_20 "Color" (Math|Conversions|ToLinearColor(Vector) "0.574409,0.582118,0.630208") :!class /Script/Engine.MaterialInstanceDynamic))
      (Utilities|Array|Clear _oldhitblocks)
      (Utilities|Array|AppendArray _oldhitblocks (Variables|Default|GetHitBlocks)))))

(fn ConstructionScript)

(fn BreakLength
  (bind _output_get (Variables|Default|Setbreak_length (+ (Variables|Default|Getbreak_length) 5e+01)))
  (if (>= _output_get 2e+03)
    (Variables|Default|SetHammering false)
    (Variables|Default|SetDrawHammerVector false)))