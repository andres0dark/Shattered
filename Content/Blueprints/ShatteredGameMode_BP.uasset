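; Game mode for local multiplayer that spawns and possesses a character for each active player on BeginPlay.
; It reads player flags from the Globals game instance and creates extra local players for active slots beyond the first.
; That same pass hands the shared camera the list of existing characters, before a second pass spawns characters at one fixed elevated point with slot index and color.
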(event EventBeginPlay
  (CallFunction|SpawnPlayers))

(event EventTick
  (params (DeltaSeconds :type Float%20%28single-precision%29)))

(fn ConstructionScript)

(fn SpawnPlayers
  (bind _asglobals (Utilities|Casting|CastToGlobals (Game|GetGameInstance)))
  (for (_array_element _array_index) (Variables|/Game/Globals.Globals_C|Getplayers _asglobals)
    (if _array_element
      (if (!= _array_index 0)
        ;[1 1 1] Add Extra Players to Game
        (Class|GameplayStatics|CreatePlayer _array_index)
        (bind _returnvalue (Actor|GetActorOfClass "/Game/Blueprints/ShatteredCamera_BP.ShatteredCamera_BP_C"))
        (bind _outactors (Actor|GetAllActorsOfClass "/Game/PlayerCharacter/ShatteredCharacter_BP.ShatteredCharacter_BP_C"))
        (Variables|/Game/Blueprints/ShatteredCamera_BP.ShatteredCamera_BP_C|Setplayers _returnvalue _outactors))))
  (for (_array_element_2 _array_index_2) (Variables|/Game/Globals.Globals_C|Getplayers _asglobals)
    (if _array_element_2
      ;[1 1 1] Spawn Character Actors and Posses
      (bind _returnvalue_2 (Game|SpawnActorfromClass "/Game/PlayerCharacter/ShatteredCharacter_BP.ShatteredCharacter_BP_C" (Math|Transform|MakeTransform "0, 0,2000.000000") "Undefined" 0 _array_index_2 (Utilities|Array|Get(acopy) (Variables|/Game/Globals.Globals_C|Getplayer_colors _asglobals) _array_index_2) 0))
      (Pawn|Possess (Game|GetPlayerController _array_index_2) _returnvalue_2))))