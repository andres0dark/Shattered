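; Main menu player controller for gamepad, handling each player's color choice and ready-up before Start opens MainMap (no ready check).
; Left stick steps through Menu entries with a re-center latch, toggling highlight images.
; On the color entry, right-stick angle rotates dial images and becomes a hue saved per controller ID in the Globals game instance.
; Confirming the last entry flags that player in Globals and freezes navigation.
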(event Input|GamepadEvents|GamepadRightX
  (params (AxisValue :type Float%20%28single-precision%29))
  (bind _returnvalue (Class|Actor|GetInputAxisKeyValue))
  (bind _returnvalue_2 (Class|Actor|GetInputAxisKeyValue))
  (bind _menu (Variables|Default|GetMenu))
  (bind _returnvalue_3 (Class|KismetMathLibrary|DegAtan2 _returnvalue _returnvalue_2))
  (bind _returnvalue_4 (+ _returnvalue_3 4.5e+02))
  (if (and (or (> (Math|Float|Absolute(Float) _returnvalue) 0.6) (> (Math|Float|Absolute(Float) _returnvalue_2) 0.6)) (== (Variables|/Game/UI/PlayerCustomization.PlayerCustomization_C|GetCurrentIndex _menu) 2))
    (Class|Widget|SetRenderTransformAngle (Variables|/Game/UI/PlayerCustomization.PlayerCustomization_C|GetImage_819 _menu) _returnvalue_4)
    (Class|Widget|SetRenderTransformAngle (Variables|/Game/UI/PlayerCustomization.PlayerCustomization_C|GetImage_947 _menu) _returnvalue_4)
    (bind _asglobals (Utilities|Casting|CastToGlobals (Game|GetGameInstance)))
    (Utilities|Array|SetArrayElem (Variables|/Game/Globals.Globals_C|Getplayer_colors _asglobals) (Class|GameplayStatics|GetPlayerControllerID self) (Class|KismetMathLibrary|HSVtoRGB (.Remainder (Math|Float|Division(WholeandRemainder) _returnvalue_4 3.6e+02)) 1.0 1.0 1.0))))

(event Input|GamepadEvents|GamepadRightY
  (params (AxisValue :type Float%20%28single-precision%29))
  (bind _returnvalue (Class|Actor|GetInputAxisKeyValue))
  (bind _returnvalue_2 (Class|Actor|GetInputAxisKeyValue))
  (bind _menu (Variables|Default|GetMenu))
  (bind _returnvalue_3 (Class|KismetMathLibrary|DegAtan2 _returnvalue _returnvalue_2))
  (bind _returnvalue_4 (+ _returnvalue_3 4.5e+02))
  (if (and (or (> (Math|Float|Absolute(Float) _returnvalue) 0.6) (> (Math|Float|Absolute(Float) _returnvalue_2) 0.6)) (== (Variables|/Game/UI/PlayerCustomization.PlayerCustomization_C|GetCurrentIndex _menu) 2))
    (Class|Widget|SetRenderTransformAngle (Variables|/Game/UI/PlayerCustomization.PlayerCustomization_C|GetImage_819 _menu) _returnvalue_4)
    (Class|Widget|SetRenderTransformAngle (Variables|/Game/UI/PlayerCustomization.PlayerCustomization_C|GetImage_947 _menu) _returnvalue_4)
    (bind _asglobals (Utilities|Casting|CastToGlobals (Game|GetGameInstance)))
    (Utilities|Array|SetArrayElem (Variables|/Game/Globals.Globals_C|Getplayer_colors _asglobals) (Class|GameplayStatics|GetPlayerControllerID self) (Class|KismetMathLibrary|HSVtoRGB (.Remainder (Math|Float|Division(WholeandRemainder) _returnvalue_4 3.6e+02)) 1.0 1.0 1.0))))

(event Input|GamepadEvents|GamepadLeftY
  (params (AxisValue :type Float%20%28single-precision%29))
  (bind _menu (Variables|Default|GetMenu))
  (bind _menu_2 (Variables|Default|GetMenu))
  (bind _menu_3 (Variables|Default|GetMenu))
  (bind _menu_4 (Variables|Default|GetMenu))
  (bind _menu_5 (Variables|Default|GetMenu))
  (bind _menu_6 (Variables|Default|GetMenu))
  (bind _menu_7 (Variables|Default|GetMenu))
  (bind _image (Variables|/Game/UI/PlayerCustomization.PlayerCustomization_C|GetImage _menu_2))
  (bind _image_1151 (Variables|/Game/UI/PlayerCustomization.PlayerCustomization_C|GetImage_1151 _menu))
  (bind _image_947 (Variables|/Game/UI/PlayerCustomization.PlayerCustomization_C|GetImage_947 _menu_4))
  (bind _image_1863 (Variables|/Game/UI/PlayerCustomization.PlayerCustomization_C|GetImage_1863 _menu_5))
  (bind _currentindex (Variables|/Game/UI/PlayerCustomization.PlayerCustomization_C|GetCurrentIndex _menu_6))
  (bind _image_2055 (Variables|/Game/UI/PlayerCustomization.PlayerCustomization_C|GetImage_2055 _menu_7))
  (if (not (Variables|Default|Getfreze_move))
    (if (> AxisValue 0.8)
      (if (Variables|Default|GetCanMove)
        (Default|SelectPrevious _menu_3)
        (Variables|Default|SetCanMove false :!label _label)
        (Utilities|FlowControl|Sequence
          (:then_0
            (if (== _currentindex 0)
              (Widget|SetVisibility _image "Hidden")
              (else
                (Widget|SetVisibility _image "Visible"))))
          (:then_1
            (if (== _currentindex 1)
              (Widget|SetVisibility _image_1151 "Hidden")
              (else
                (Widget|SetVisibility _image_1151 "Visible"))))
          (:then_2
            (if (== _currentindex 2)
              (Widget|SetVisibility _image_947 "Hidden")
              (else
                (Widget|SetVisibility _image_947 "Visible"))))
          (:then_3
            (if (== _currentindex 3)
              (Widget|SetVisibility _image_1863 "Hidden")
              (Widget|SetVisibility _image_2055 "Hidden")
              (else
                (Widget|SetVisibility _image_1863 "Visible")
                (Widget|SetVisibility _image_2055 "Visible"))))))
      (elif (<= AxisValue -0.8)
        (if (Variables|Default|GetCanMove)
          (Default|SelectNext _menu_3)
          (goto _label))
        (elif (<= (Math|Float|Absolute(Float) AxisValue) 0.5)
          (Variables|Default|SetCanMove true))))))

(event Input|GamepadEvents|GamepadFaceButtonBottom
  (params (Key :type Key%20Structure :default "None"))
  (bind _menu (Variables|Default|GetMenu))
  (:Pressed
    (if (== (Variables|/Game/UI/PlayerCustomization.PlayerCustomization_C|GetCurrentIndex (Variables|Default|GetMenu)) 3)
      (Widget|SetVisibility (Variables|/Game/UI/PlayerCustomization.PlayerCustomization_C|GetImage_2483 _menu) "Visible")
      (Widget|SetVisibility (Variables|/Game/UI/PlayerCustomization.PlayerCustomization_C|GetImage_2308 _menu) "Hidden")
      (Variables|Default|Setfreze_move true)
      (bind _asglobals (Utilities|Casting|CastToGlobals (Game|GetGameInstance)))
      (Utilities|Array|SetArrayElem (Variables|/Game/Globals.Globals_C|Getplayers _asglobals) (Class|GameplayStatics|GetPlayerControllerID self) true true))))

(event Input|GamepadEvents|GamepadSpecialRight
  (params (Key :type Key%20Structure :default "None"))
  (:Pressed
    (Game|OpenLevel(byName) "MainMap")))

(fn ConstructionScript)