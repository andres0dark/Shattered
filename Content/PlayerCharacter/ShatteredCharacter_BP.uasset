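; ShatteredCharacter_BP is a player-specific shattered character actor that colors and positions itself when play begins.
; SetColor creates a dynamic material on the mesh's first slot and sets its Color parameter to PlayerColor.
; SpawnFunction then finds the PlayerStart tagged "player" plus PlayerInt, saves its transform as SpawnLocation and teleports the actor there.
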(event EventBeginPlay
  (CallFunction|SetColor)
  (CallFunction|SpawnFunction))

(fn ConstructionScript)

(fn SpawnFunction
  (bind _outactors (Actor|GetAllActorsOfClass "/Script/Engine.PlayerStart"))
  (for _array_element _outactors
    (if (Utilities|Enum|Equal(Enum) (Utilities|Text|ToText(Name) (Variables|/Script/Engine.PlayerStart|GetPlayerStartTag _array_element)) (Utilities|Text|ToText(String) (Utilities|String|Append "player" (Utilities|String|ToString(Integer) (Variables|Default|GetPlayerInt)))))
      (bind _output_get (Variables|Default|SetSpawnLocation (Transformation|GetActorTransform _array_element)))
      (Transformation|SetActorTransform _output_get false true))))

(fn SetColor
  (bind _returnvalue (Rendering|Material|CreateDynamicMaterialInstance (Variables|Character|GetMesh) 0 0 "None" :!class /Script/Engine.PrimitiveComponent))
  (Rendering|Material|SetVectorParameterValue _returnvalue "Color" (Variables|Default|GetPlayerColor) :!class /Script/Engine.MaterialInstanceDynamic))